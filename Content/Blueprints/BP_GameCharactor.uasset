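; BP_GameCharactor is a player character Blueprint providing basic movement, look and jump controls.
; Input axes drive controller yaw and pitch, while forward and right movement follow the full control rotation's vectors.
; The Jump action triggers a jump on press, with no release handler, and the construction script is empty.
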(event Input|ActionEvents|InputActionJump
  (params (Key :type Key%20Structure :default "None"))
  ;[1 1 1] Charactor Jump
  (:Pressed
    (Character|Jump)))

(event Input|AxisEvents|InputAxisMoveForward
  (params (AxisValue :type Float%20%28single-precision%29))
  ;[1 1 1] Charactor Movement
  (Pawn|Input|AddMovementInput (Math|Vector|GetForwardVector (Pawn|GetControlRotation :!class /Script/Engine.Pawn)) AxisValue false))

(event Input|AxisEvents|InputAxisRotationX
  (params (AxisValue :type Float%20%28single-precision%29))
  ;[1 1 1] Charactor Rotation
  (Pawn|Input|AddControllerYawInput AxisValue))

(event Input|AxisEvents|InputAxisRotationY
  (params (AxisValue :type Float%20%28single-precision%29))
  ;[1 1 1] Charactor Rotation
  (Pawn|Input|AddControllerPitchInput AxisValue))

(event Input|AxisEvents|InputAxisMoveRight
  (params (AxisValue :type Float%20%28single-precision%29))
  ;[1 1 1] Charactor Movement
  (Pawn|Input|AddMovementInput (Math|Vector|GetRightVector (Pawn|GetControlRotation :!class /Script/Engine.Pawn)) AxisValue false))

(fn ConstructionScript)